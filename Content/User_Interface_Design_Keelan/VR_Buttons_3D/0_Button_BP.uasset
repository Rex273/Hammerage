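; A 3D button Blueprint, filed under VR buttons, that sinks while an actor overlaps its Box and rises when clear.
; Each Tick polls the Box's overlapping actors and steps ButtonRed's relative Z down or up, clamped between zero and ButtonOffset.
; MoveComponentTo applies each step over a near-zero duration, so travel speed depends on frame rate.
; It contains only the motion, with no press event or triggered action.
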(event EventTick
  (params (DeltaSeconds :type Float%20%28single-precision%29))
  (bind _button_red (Variables|Default|GetButton_Red))
  (if (> (Utilities|Array|Length (Collision|GetOverlappingActors (Variables|Default|GetBox) 0 :!class /Script/Engine.PrimitiveComponent)) 0)
    (Components|MoveComponentTo _button_red (Math|Vector|MakeVector 0.0 0.0 (Math|Float|Clamp(Float) (- (.z (Variables|/Script/Engine.SceneComponent|GetRelativeLocation _button_red)) 2.0) 0.0 (Variables|Default|GetButton%20Offset))) "0, 0, 0" false false 0.0001 false)
    (else
      (Components|MoveComponentTo 0 (Math|Vector|MakeVector 0.0 0.0 (Math|Float|Clamp(Float) (+ (.z (Variables|/Script/Engine.SceneComponent|GetRelativeLocation (Variables|Default|GetButton_Red))) 2.0) 0.0 (Variables|Default|GetButton%20Offset))) "0, 0, 0" false false 0.0001 false))))

(fn ConstructionScript)