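; CookieCutter is a shape-fitting puzzle Blueprint with cube, arrow, hexagon and triangle slots.
; Overlap events on each shape's component set its fit flag and turn its mesh green, or clear the flag and turn it red when the overlap ends.
; Tick polls the four flags and sets NextDoor to true once all fit; nothing here resets it or checks which actor overlaps.
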(event OnComponentBeginOverlap(Box)
  (params (OverlappedComponent :type Primitive%20Component%20Object%20Reference) (OtherActor :type Actor%20Object%20Reference) (OtherComp :type Primitive%20Component%20Object%20Reference) (OtherBodyIndex :type Integer) (bFromSweep :type Boolean) (SweepResult :type Hit%20Result%20Structure%20%28by%20ref%29))
  (Rendering|Material|SetMaterial (Variables|Default|GetCubeMesh) 0 "/AnimationSharing/AnimSharingGreen.AnimSharingGreen")
  (Variables|Default|SetCubeFit true))

(event OnComponentEndOverlap(Box)
  (params (OverlappedComponent :type Primitive%20Component%20Object%20Reference) (OtherActor :type Actor%20Object%20Reference) (OtherComp :type Primitive%20Component%20Object%20Reference) (OtherBodyIndex :type Integer))
  (Rendering|Material|SetMaterial (Variables|Default|GetCubeMesh) 0 "/AnimationSharing/AnimSharingRed.AnimSharingRed")
  (Variables|Default|SetCubeFit false))

(event OnComponentBeginOverlap(Arrow)
  (params (OverlappedComponent :type Primitive%20Component%20Object%20Reference) (OtherActor :type Actor%20Object%20Reference) (OtherComp :type Primitive%20Component%20Object%20Reference) (OtherBodyIndex :type Integer) (bFromSweep :type Boolean) (SweepResult :type Hit%20Result%20Structure%20%28by%20ref%29))
  (Rendering|Material|SetMaterial (Variables|Default|GetArrowMesh1) 0 "/AnimationSharing/AnimSharingGreen.AnimSharingGreen")
  (Variables|Default|SetArrowFit true))

(event OnComponentEndOverlap(Arrow)
  (params (OverlappedComponent :type Primitive%20Component%20Object%20Reference) (OtherActor :type Actor%20Object%20Reference) (OtherComp :type Primitive%20Component%20Object%20Reference) (OtherBodyIndex :type Integer))
  (Rendering|Material|SetMaterial (Variables|Default|GetArrowMesh1) 0 "/AnimationSharing/AnimSharingRed.AnimSharingRed")
  (Variables|Default|SetArrowFit false))

(event OnComponentBeginOverlap(Hexagon)
  (params (OverlappedComponent :type Primitive%20Component%20Object%20Reference) (OtherActor :type Actor%20Object%20Reference) (OtherComp :type Primitive%20Component%20Object%20Reference) (OtherBodyIndex :type Integer) (bFromSweep :type Boolean) (SweepResult :type Hit%20Result%20Structure%20%28by%20ref%29))
  (Rendering|Material|SetMaterial (Variables|Default|GetHexMesh2) 0 "/AnimationSharing/AnimSharingGreen.AnimSharingGreen")
  (Variables|Default|SetHexFit true))

(event OnComponentEndOverlap(Hexagon)
  (params (OverlappedComponent :type Primitive%20Component%20Object%20Reference) (OtherActor :type Actor%20Object%20Reference) (OtherComp :type Primitive%20Component%20Object%20Reference) (OtherBodyIndex :type Integer))
  (Rendering|Material|SetMaterial (Variables|Default|GetHexMesh2) 0 "/AnimationSharing/AnimSharingRed.AnimSharingRed")
  (Variables|Default|SetHexFit false))

(event OnComponentBeginOverlap(Triangle)
  (params (OverlappedComponent :type Primitive%20Component%20Object%20Reference) (OtherActor :type Actor%20Object%20Reference) (OtherComp :type Primitive%20Component%20Object%20Reference) (OtherBodyIndex :type Integer) (bFromSweep :type Boolean) (SweepResult :type Hit%20Result%20Structure%20%28by%20ref%29))
  (Rendering|Material|SetMaterial (Variables|Default|GetTriangleMesh3) 0 "/AnimationSharing/AnimSharingGreen.AnimSharingGreen")
  (Variables|Default|SetTriangleFit true))

(event OnComponentEndOverlap(Triangle)
  (params (OverlappedComponent :type Primitive%20Component%20Object%20Reference) (OtherActor :type Actor%20Object%20Reference) (OtherComp :type Primitive%20Component%20Object%20Reference) (OtherBodyIndex :type Integer))
  (Rendering|Material|SetMaterial (Variables|Default|GetTriangleMesh3) 0 "/AnimationSharing/AnimSharingRed.AnimSharingRed")
  (Variables|Default|SetTriangleFit false))

(event EventTick
  (params (DeltaSeconds :type Float%20%28single-precision%29))
  (if (and (Variables|Default|GetCubeFit) (Variables|Default|GetArrowFit))
    (if (and (Variables|Default|GetHexFit) (Variables|Default|GetTriangleFit))
      (Variables|Default|SetNextDoor true))))

(fn ConstructionScript)