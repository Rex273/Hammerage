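; Golden ticket pickup actor that counts toward unlocking the elevator door.
; Any overlap with its Cube increments its TicketCount variable, then destroys the actor after a short delay.
; Tick polls that count every frame and, when it equals four, finds the ElevatorDoor actor by class and sets its Unlocked flag.
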(event OnComponentBeginOverlap(Cube)
  (params (OverlappedComponent :type Primitive%20Component%20Object%20Reference) (OtherActor :type Actor%20Object%20Reference) (OtherComp :type Primitive%20Component%20Object%20Reference) (OtherBodyIndex :type Integer) (bFromSweep :type Boolean) (SweepResult :type Hit%20Result%20Structure%20%28by%20ref%29))
  (Variables|Default|SetTicketCount (+ (Variables|Default|GetTicketCount) 1.0))
  (Utilities|FlowControl|Delay 0.8)
  (Actor|DestroyActor))

(event Collision|EventActorBeginOverlap
  (params (OtherActor :type Actor%20Object%20Reference)))

(event EventTick
  (params (DeltaSeconds :type Float%20%28single-precision%29))
  (if (== (Variables|Default|GetTicketCount) 4.0)
    (bind _returnvalue (Actor|GetActorOfClass "/Game/Blueprints/KIERAN/OTHER/ElevatorDoor.ElevatorDoor_C"))
    (Variables|/Game/Blueprints/KIERAN/OTHER/ElevatorDoor.ElevatorDoor_C|SetUnlocked _returnvalue true)))

(fn ConstructionScript)