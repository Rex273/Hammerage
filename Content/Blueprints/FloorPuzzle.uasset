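; FloorPuzzle is a floor puzzle Blueprint that sets an Open flag once all four of its trigger boxes have been overlapped.
; Each box's begin-overlap event swaps its matching Right mesh to the Impacted material and latches its Break boolean, with no filter on the overlapping actor.
; Tick polls the four booleans to set Open; nothing in this graph resets them or acts on Open.
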(event OnComponentBeginOverlap(Box2)
  (params (OverlappedComponent :type Primitive%20Component%20Object%20Reference) (OtherActor :type Actor%20Object%20Reference) (OtherComp :type Primitive%20Component%20Object%20Reference) (OtherBodyIndex :type Integer) (bFromSweep :type Boolean) (SweepResult :type Hit%20Result%20Structure%20%28by%20ref%29))
  (Rendering|Material|SetMaterial (Variables|Default|GetRight2) 0 "/Game/Blueprints/Impacted.Impacted")
  (Variables|Default|SetBreak2 true))

(event OnComponentBeginOverlap(Box1)
  (params (OverlappedComponent :type Primitive%20Component%20Object%20Reference) (OtherActor :type Actor%20Object%20Reference) (OtherComp :type Primitive%20Component%20Object%20Reference) (OtherBodyIndex :type Integer) (bFromSweep :type Boolean) (SweepResult :type Hit%20Result%20Structure%20%28by%20ref%29))
  (Rendering|Material|SetMaterial (Variables|Default|GetRight1) 0 "/Game/Blueprints/Impacted.Impacted")
  (Variables|Default|SetBreak1 true))

(event OnComponentBeginOverlap(Box4)
  (params (OverlappedComponent :type Primitive%20Component%20Object%20Reference) (OtherActor :type Actor%20Object%20Reference) (OtherComp :type Primitive%20Component%20Object%20Reference) (OtherBodyIndex :type Integer) (bFromSweep :type Boolean) (SweepResult :type Hit%20Result%20Structure%20%28by%20ref%29))
  (Rendering|Material|SetMaterial (Variables|Default|GetRight4) 0 "/Game/Blueprints/Impacted.Impacted")
  (Variables|Default|SetBreak4 true))

(event OnComponentBeginOverlap(Box3)
  (params (OverlappedComponent :type Primitive%20Component%20Object%20Reference) (OtherActor :type Actor%20Object%20Reference) (OtherComp :type Primitive%20Component%20Object%20Reference) (OtherBodyIndex :type Integer) (bFromSweep :type Boolean) (SweepResult :type Hit%20Result%20Structure%20%28by%20ref%29))
  (Rendering|Material|SetMaterial (Variables|Default|GetRight3) 0 "/Game/Blueprints/Impacted.Impacted")
  (Variables|Default|SetBreak3 true))

(event EventTick
  (params (DeltaSeconds :type Float%20%28single-precision%29))
  (if (Math|Boolean|ANDBoolean (Variables|Default|GetBreak1) (Variables|Default|GetBreak2) (Variables|Default|GetBreak3) (Variables|Default|GetBreak4))
    (Variables|Default|SetOpen true)))

(fn ConstructionScript)